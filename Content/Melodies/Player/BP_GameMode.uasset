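; Game mode for a Five Nights at Freddy's-style night shift, running the clock, power drain and night progression.
; A looping timer advances the hour until the finish time, then shows the night-complete widget, increments the saved night in the GameInstance and reloads, or returns to the menu after night five.
; Power drains in a delayed self-calling loop that branches on camera mode, updating the player's HUD.
; Running out of power only prints a message.
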(event `self.ReceiveBeginPlay`
  (bind _asbp_game_instances (cast `/Game/Melodies/Player/BP_GameInstances` (`GameplayStatics.GetGameInstance`)))
  (set `self.Game Instances` _asbp_game_instances)
  (bind _asbp_player (cast `/Game/Melodies/Player/BP_Player` (`GameplayStatics.GetPlayerPawn` 0)))
  (set `self.BP Player` _asbp_player)
  (`KismetSystemLibrary.Delay` 0.2)
  (`TextBlock.SetText` (`/Game/Melodies/Widgets/Player/W_PlayerView.Text_Night` (`/Game/Melodies/Player/BP_Player.Player View` (`self.BP Player`))) (`|FormatText` "NIGHT {Night}" (`KismetTextLibrary.Conv_IntToText` (`/Game/Melodies/Player/BP_GameInstances.CurrentNight` (`self.Game Instances`)) false false)))
  (`self.UpdateTimeWidget`)
  (`KismetSystemLibrary.K2_SetTimer` null "UpdateClock" (`self.TimeRate`) true)
  (set `self.CurrentPower` (`self.MaxPower`))
  (`KismetSystemLibrary.Delay` 0.4)
  (`self.RemovePower`))

(event `UpdateClock`
  (bind _game_instances (`self.Game Instances`))
  (bind _game_instances_2 (`self.Game Instances`))
  (set `self.CurrentTime` (+ (`self.CurrentTime`) 1))
  (if (> (`self.CurrentTime`) 12)
    (set `self.CurrentTime` 1))
  (`self.UpdateTimeWidget`)
  (if (== (`self.CurrentTime`) (`self.FinishTime`))
    (`KismetSystemLibrary.PrintString` "YOU WIN -> Go to next night")
    (`KismetSystemLibrary.K2_ClearTimer` null "UpdateClock")
    (bind _returnvalue (`|CreateWidget` "/Game/Melodies/Widgets/W_NightComplete.W_NightComplete_C"))
    (`UserWidget.AddToViewport` _returnvalue 0)
    (set `/Game/Melodies/Player/BP_GameInstances.CurrentNight` (+ (`/Game/Melodies/Player/BP_GameInstances.CurrentNight` _game_instances_2) 1) _game_instances_2)
    (`KismetSystemLibrary.Delay` 2.0)
    (if (>= (`/Game/Melodies/Player/BP_GameInstances.CurrentNight` _game_instances) 6)
      (`KismetSystemLibrary.PrintString` "ALL NIGHTS COMPLETED - GAME COMPLETED")
      (`GameplayStatics.SetGamePaused` true)
      (`GameplayStatics.OpenLevelBySoftObjectPtr` "/Game/Melodies/Maps/Menu_Screen.Menu_Screen")
      (set `/Game/Melodies/Player/BP_GameInstances.MainNightsComplete` true _game_instances)
      (else
        (`GameplayStatics.OpenLevelBySoftObjectPtr` "/Game/Gameplay/Maps/Test.Test")))))

(event `Update Time Widget`
  (`TextBlock.SetText` (`/Game/Melodies/Widgets/Player/W_PlayerView.Text_Time` (`/Game/Melodies/Player/BP_Player.Player View` (`self.BP Player`))) (`|FormatText` "{Time} AM" (`KismetTextLibrary.Conv_IntToText` (`self.CurrentTime`) false false))))

(event `Remove Power`
  (`self.AdjustPower` (`self.RemovePowerValue`)))

(event `Remove Power Camera`
  (`self.AdjustPower` (`self.RemovePowerValueCam`)))

(event `Remove Power Generator`
  (`self.AdjustPower` (`self.RemovePowerValueGenerator`)))

(event `Adjust Power`
  (params (Amount :type "Float (double-precision)"))
  (set `self.CurrentPower` (`KismetMathLibrary.FClamp` (- (`self.CurrentPower`) Amount)))
  (`TextBlock.SetText` (`/Game/Melodies/Widgets/Player/W_PlayerView.Text_Power` (`/Game/Melodies/Player/BP_Player.Player View` (`self.BP Player`))) (`|FormatText` "Power: {Power}%" (`KismetMathLibrary.Conv_IntToDouble` (`KismetMathLibrary.Round` (* (/ (`self.CurrentPower`) (`self.MaxPower`)) 100.0)))))
  (if (<= (`self.CurrentPower`) 0.0)
    (`KismetSystemLibrary.PrintString` "Power Off")
    (elif (`/Game/Melodies/Player/BP_Player.CamMode` (`self.BP Player`))
      ;[1 1 1] Remove Power - If On Camares
      (`KismetSystemLibrary.Delay` 0.2)
      (`self.Remove Power Cam`)
      (else
        ;[1 1 1] Remove Power - The rate will bepend on night number
        (`KismetSystemLibrary.Delay` 0.2)
        (`self.RemovePower`)))))

(event `AdjustPower`
  (params (Amount :type "Float (double-precision)")))

(event `RemovePower`)

(event `Remove Power Cam`)

(fn `UpdateTimeWidget`)

(fn `UserConstructionScript`)