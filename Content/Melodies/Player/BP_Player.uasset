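; BP_Player is the player Blueprint for an animatronic game with a fixed-position look-around view, camera mode and shock action.
; BeginPlay adds Enhanced Input mapping, shows the cursor, clamps camera angles and creates the front and general view widgets.
; Helpers create directional view widgets, while TurnCamera applies yaw and pitch from turn variables.
; Shock briefly sets a flag in camera mode, PowerOff restores the player view and clears widgets, and Exit opens the main menu.
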(event `self.ReceiveBeginPlay`
  (bind _returnvalue (`GameplayStatics.GetPlayerCameraManager` 0))
  (bind _asplayer_controller (cast `PlayerController` (`self.GetController`)))
  (bind _returnvalue_2 (pcsubsystem `EnhancedInputLocalPlayerSubsystem` _asplayer_controller))
  (`/Engine/EditorBlueprintResources/StandardMacros.IsValid` _returnvalue_2
    (:`Is Valid`
      (`EnhancedInputSubsystemInterface.AddMappingContext` _returnvalue_2 "/Game/Melodies/Player/Input/Player_Default.Player_Default" 0 (struct))
      (set `PlayerController.bShowMouseCursor` true (`GameplayStatics.GetPlayerController` 0))
      (set `PlayerCameraManager.ViewYawMin` -60.0 _returnvalue)
      (set `PlayerCameraManager.ViewYawMax` 60.0 _returnvalue)
      (set `PlayerCameraManager.ViewPitchMin` 0.0 _returnvalue)
      (set `PlayerCameraManager.ViewPitchMax` 90.0 _returnvalue)
      (bind _asbp_game_mode (cast `/Game/Melodies/Player/BP_GameMode` (`GameplayStatics.GetGameMode`)))
      (set `self.BP Game Mode` _asbp_game_mode)
      (`/Engine/EditorBlueprintResources/StandardMacros.IsValid` (`self.Animatronic Base`)
        (:`Is Valid`
          (bind _asbp_animatronic_base (cast `/Game/Melodies/Animatronics/BP_AnimatronicBase` (`GameplayStatics.GetPlayerCharacter` 0)))
          (set `self.Animatronic Base` _asbp_animatronic_base))
        (:`Is Not Valid`
          _))
      (`self.FrontView`)
      (`self.PlayerView`))))

(event `TurnCamera`
  (`self.AddControllerYawInput` (`self.TurnPlayerSide`))
  (`self.AddControllerPitchInput` (`self.TurnPlayerUp`)))

(event `PowerOff`
  (`PlayerController.SetViewTargetWithBlend` (`GameplayStatics.GetPlayerController` 0) self 0.0 "VTBlend_Linear" 0.0 false)
  (`WidgetLayoutLibrary.RemoveAllWidgets`))

(event `EnhancedInput|/Game/Melodies/Player/Input/Actions/Player_Shock`
  (params (ActionValue :type Boolean) (ElapsedSeconds :type "Float (double-precision)") (TriggeredSeconds :type "Float (double-precision)") (InputAction :type "InputAction Object Reference" :default "/Game/Melodies/Player/Input/Actions/Player_Shock.Player_Shock"))
  (:`Started`
    (if (`self.CamMode`)
      (set `self.IsShocking` true)
      (`KismetSystemLibrary.PrintString` "Shocked")
      (`KismetSystemLibrary.Delay` 1.0)
      (set `self.IsShocking` false))))

(event `EnhancedInput|/Game/Melodies/Player/Input/Actions/Player_Exit`
  (params (ActionValue :type Boolean) (ElapsedSeconds :type "Float (double-precision)") (TriggeredSeconds :type "Float (double-precision)") (InputAction :type "InputAction Object Reference" :default "/Game/Melodies/Player/Input/Actions/Player_Exit.Player_Exit"))
  (:`Started`
    (`GameplayStatics.OpenLevelBySoftObjectPtr` "/Game/Melodies/Maps/M_MainMenu.M_MainMenu")))

(fn `FrontView`
  (returns (ReturnValue :type "/Game/Melodies/Widgets/Player/W_PlayerViewFront Object Reference"))
  (bind _returnvalue (`|CreateWidget` "/Game/Melodies/Widgets/Player/W_PlayerViewFront.W_PlayerViewFront_C"))
  (bind _output_get (set `self.Player Front View` _returnvalue))
  (`UserWidget.AddToViewport` _output_get 0)
  (return _output_get))

(fn `LeftView`
  (bind _returnvalue (`|CreateWidget` "/Game/Melodies/Widgets/Player/W_PlayerViewLeft.W_PlayerViewLeft_C"))
  (bind _output_get (set `self.Player Left View` _returnvalue))
  (`UserWidget.AddToViewport` _output_get 0))

(fn `PlayerView`
  (returns (ReturnValue :type "/Game/Melodies/Widgets/Player/W_PlayerView Object Reference"))
  (bind _returnvalue (`|CreateWidget` "/Game/Melodies/Widgets/Player/W_PlayerView.W_PlayerView_C"))
  (bind _output_get (set `self.Player View` _returnvalue))
  (`UserWidget.AddToViewport` _output_get 0)
  (return _output_get))

(fn `RightView`
  (bind _returnvalue (`|CreateWidget` "/Game/Melodies/Widgets/Player/W_PlayerViewRight.W_PlayerViewRight_C"))
  (bind _output_get (set `self.Player Right View` _returnvalue))
  (`UserWidget.AddToViewport` _output_get 0))

(fn `Test`
  (returns (ReturnValue :type "/Game/Melodies/Widgets/W_Test Object Reference"))
  (bind _returnvalue (`|CreateWidget` "/Game/Melodies/Widgets/W_Test.W_Test_C"))
  (bind _output_get (set `self.Player Test` _returnvalue))
  (`UserWidget.AddToViewport` _output_get 0)
  (return _output_get))

(fn `TopView`
  (bind _returnvalue (`|CreateWidget` "/Game/Melodies/Widgets/Player/W_PlayerViewTop.W_PlayerViewTop_C"))
  (bind _output_get (set `self.Player Top View` _returnvalue))
  (`UserWidget.AddToViewport` _output_get 0))

(fn `UserConstructionScript`)