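; BP_SecurityCamera is a security camera actor that the player's view can switch to.
; On BeginPlay, if CanRotate is set, it plays the CamRotate timeline after a short delay.
; The timeline's update graph lerps the camera's relative yaw between Max and Min, with pitch and roll fixed at zero.
; SwitchToCamera makes this actor the first player controller's view target.
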(event `self.ReceiveBeginPlay`
  (if (`self.CanRotate`)
    (`KismetSystemLibrary.Delay` 0.2)
    (`TimelineComponent.Play` (`self.CamRotate`))))

(event `Switch To Camera`
  (`PlayerController.SetViewTargetWithBlend` (`GameplayStatics.GetPlayerController` 0) self 0.0 "VTBlend_Linear" 0.0 false))

(fn `UserConstructionScript`)