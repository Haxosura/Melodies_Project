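; Base animatronic for a night-based game with cameras, active from its start night when difficulty is above zero.
; On BeginPlay it starts a looping AI MoveTo patrol through target points, with waits scaled by speed and difficulty.
; If the player is in camera mode as it moves, static flashes on their view.
; The last point only prints an attack, then it returns to start, optionally visits the generator, and repeats.
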(event `self.ReceiveBeginPlay`
  (bind _targetlocation (`self.TargetLocation`))
  (bind _output (`|GetArrayItem` (`self.TargetPoints`) (`self.TargetLocation`)))
  (bind _asbp_game_instances (cast `/Game/Melodies/Player/BP_GameInstances` (`GameplayStatics.GetGameInstance`)))
  (set `self.GameInstance` _asbp_game_instances)
  (bind _asbp_player (cast `/Game/Melodies/Player/BP_Player` (`GameplayStatics.GetPlayerPawn` 0)))
  (set `self.BP Player` _asbp_player)
  (if (>= (`/Game/Melodies/Player/BP_GameInstances.CurrentNight` (`self.GameInstance`)) (`self.StartNight`))
    (if (not (<= (`self.Difficlty`) 0))
      (`KismetSystemLibrary.PrintString` (`KismetTextLibrary.Conv_TextToString` (`|FormatText` "Active {X}" (`KismetSystemLibrary.GetDisplayName` self))))
      (`KismetSystemLibrary.Delay` (/ (`self.MovementSpeed`) (* (`self.Difficlty`) (`self.MoveMult`))))
      (bind _output_get (set `self.TargetLenght` (`KismetArrayLibrary.Array_Length` (`self.TargetPoints`))))
      (`KismetSystemLibrary.PrintString` (`KismetTextLibrary.Conv_TextToString` (`|FormatText` "{Y} Target Lenght {X}" (`KismetSystemLibrary.GetDisplayName` self) _output_get)))
      (if (`/Game/Melodies/Player/BP_Player.CamMode` (`self.BP Player`))
        (set `self.MovementStatic` true)
        (bind _static_image (`self.Static Flash`))
        (`|ExecutionSequence`
          (:`then_0`
            (`KismetSystemLibrary.Delay` 2.0)
            (`Widget.SetVisibility` _static_image "Hidden"))
          (:`then_1`
            (`|AIMoveTo` self (0.0 0.0 0.0) _output :!label _label
              (:`OnSuccess`
                (set `self.MovementStatic` false)
                (set `self.TargetLocation` (+ _targetlocation 1))
                (`KismetSystemLibrary.PrintString` (`KismetTextLibrary.Conv_TextToString` (`|FormatText` "{Y} Location {X}" (`KismetSystemLibrary.GetDisplayName` self) (`KismetSystemLibrary.GetDisplayName` _output))))
                (if (>= _targetlocation (`self.TargetLenght`))
                  (set `self.TargetLocation` 0)
                  (`KismetSystemLibrary.PrintString` (`KismetTextLibrary.Conv_TextToString` (`|FormatText` "{Y} Attacked" (`KismetSystemLibrary.GetObjectName` self))))
                  (`KismetSystemLibrary.Delay` 2.0)
                  (`|AIMoveTo` self (0.0 0.0 0.0) (`self.Start Point`)
                    (:`OnSuccess`
                      (if (`self.AttackGenerator`)
                        (`|AIMoveTo` self (0.0 0.0 0.0) (`self.Generator`)
                          (:`OnSuccess`
                            (goto _label)))
                        (else
                          (goto _label)))))
                  (else
                    (`KismetSystemLibrary.Delay` (/ (`self.MovementSpeed`) (* (`self.Difficlty`) (`self.MoveMult`))))
                    (if (`/Game/Melodies/Player/BP_Player.CamMode` (`self.BP Player`))
                      (set `self.MovementStatic` true)
                      (bind _static_image_2 (`self.Static Flash`))
                      (`|ExecutionSequence`
                        (:`then_0`
                          (`KismetSystemLibrary.Delay` 2.0)
                          (`Widget.SetVisibility` _static_image_2 "Hidden"))
                        (:`then_1`
                          (set `self.MovementStatic` false :!label _label_2)
                          (goto _label)))
                      (else
                        (goto _label_2))))))
              (:`OnFail`
                (`KismetSystemLibrary.PrintString` (`KismetTextLibrary.Conv_TextToString` (`|FormatText` "{Y} Movement Failed" (`KismetSystemLibrary.GetDisplayName` self))))))))
        (else
          (goto _label))))))

(fn `Static Flash`
  (returns (Static_Image :type "Image Object Reference"))
  (bind _player_front_view (`/Game/Melodies/Player/BP_Player.Player Front View` (`self.BP Player`)))
  (bind _static_image (`/Game/Melodies/Widgets/Player/W_PlayerViewFront.Static_Image` _player_front_view))
  (`Widget.SetVisibility` _static_image "Visible")
  (`UserWidget.PlayAnimation` _player_front_view (`/Game/Melodies/Widgets/Player/W_PlayerViewFront.Static` _player_front_view) 0.0 1 "Forward" 1.0 false)
  (return _static_image))

(fn `UserConstructionScript`)